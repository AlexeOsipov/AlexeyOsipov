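; Player controller that owns the main HUD and feeds it the player character's health and interaction prompt.
; On BeginPlay it creates the MainWindow widget and caches the controlled MainCharacter.
; Each Tick it pushes current and max HP to the widget, then sets the prompt by polling the character's references.
; An interactable weapon shows its display name and takes priority over a lamp's "Activate"; otherwise the prompt is blank.
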(event EventBeginPlay
  (Utilities|FlowControl|Sequence
    (:then_0
      (bind _returnvalue (UserInterface|CreateWidget "/Game/AlexeyOsipov/UIX/MainWindow.MainWindow_C"))
      (Variables|Default|SetMainWindow _returnvalue)
      (UserInterface|Viewport|AddtoViewport (Variables|Default|GetMainWindow) 0))
    (:then_1
      (bind _asmain_character (Utilities|Casting|CastToMainCharacter (Pawn|GetControlledPawn)))
      (Variables|Default|SetMyPawnRef _asmain_character))))

(event EventTick
  (params (DeltaSeconds :type Float%20%28single-precision%29))
  (bind _mypawnref (Variables|Default|GetMyPawnRef))
  (bind _weaponrefinteract (Variables|/Game/AlexeyOsipov/BluePrints/Character/MainCharacter.MainCharacter_C|GetWeaponRefInteract _mypawnref))
  (Utilities|FlowControl|Sequence
    (:then_0
      (|SetHP))
    (:then_1
      (if (Utilities|IsValid (Variables|/Game/AlexeyOsipov/BluePrints/Character/MainCharacter.MainCharacter_C|GetWeaponRefInteract (Variables|Default|GetMyPawnRef)))
        (if (Utilities|IsValid _weaponrefinteract)
          (Default|UpdateInteractinfo (Variables|Default|GetMainWindow) (Utilities|Text|ToText(String) (Utilities|GetDisplayName _weaponrefinteract))))
        (elif (Utilities|IsValid (Variables|/Game/AlexeyOsipov/BluePrints/Character/MainCharacter.MainCharacter_C|GetLampreference (Variables|Default|GetMyPawnRef)))
          (Default|UpdateInteractinfo (Variables|Default|GetMainWindow) "Activate")
          (else
            (Default|UpdateInteractinfo (Variables|Default|GetMainWindow))))))))

(fn ConstructionScript)