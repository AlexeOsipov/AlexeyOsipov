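; Player character Blueprint with axis-driven movement and look, jump, sprint, and a simple health pool shown on a text render and debug print.
; Capsule overlaps cache nearby BaseLamp and BaseWeapon references, which Interact uses to toggle the lamp or swap weapons.
; Weapons attach to a scene component with physics off, fire on input, and detach with physics on when dropped.
; Damage clamps health, only printing a death message at zero.
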(event OnComponentEndOverlap(CapsuleComponent)
  (params (OverlappedComponent :type Primitive%20Component%20Object%20Reference) (OtherActor :type Actor%20Object%20Reference) (OtherComp :type Primitive%20Component%20Object%20Reference) (OtherBodyIndex :type Integer))
  (Utilities|FlowControl|Sequence
    (:then_0
      ;[1 1 1] Уточнение типа данных
      (bind _asbase_lamp (Utilities|Casting|CastToBaseLamp OtherActor))
      (if true
        (Variables|Default|SetLampreference 0)))
    (:then_1
      (bind _asbase_weapon (Utilities|Casting|CastToBaseWeapon OtherActor))
      (if true
        (Variables|Default|SetWeaponRefInteract 0)))))

(event OnComponentBeginOverlap(CapsuleComponent)
  (params (OverlappedComponent :type Primitive%20Component%20Object%20Reference) (OtherActor :type Actor%20Object%20Reference) (OtherComp :type Primitive%20Component%20Object%20Reference) (OtherBodyIndex :type Integer) (bFromSweep :type Boolean) (SweepResult :type Hit%20Result%20Structure%20%28by%20ref%29))
  (Utilities|FlowControl|Sequence
    (:then_0
      ;[1 1 1] Уточнение типа данных
      (bind _asbase_lamp (Utilities|Casting|CastToBaseLamp OtherActor))
      (Variables|Default|SetLampreference _asbase_lamp))
    (:then_1
      (bind _asbase_weapon (Utilities|Casting|CastToBaseWeapon OtherActor))
      (Variables|Default|SetWeaponRefInteract _asbase_weapon))))

(event Custom|InitCharactor
  (Variables|Default|SetHP_Current (Variables|Default|GetHP_Max)))

(event EventBeginPlay
  (CallFunction|InitCharactor))

(event Collision|EventActorBeginOverlap
  (params (OtherActor :type Actor%20Object%20Reference)))

(event EventTick
  (params (DeltaSeconds :type Float%20%28single-precision%29))
  (Development|PrintString (Utilities|String|Append (Utilities|GetDisplayName 0) ": [" (Utilities|String|ToString(Float) (Variables|Default|GetHP_Current)) "]") true true "(R=0.000000,G=0.660000,B=1.000000,A=1.000000)" 0.0)
  (Rendering|Components|TextRender|SetText (Variables|Default|GetTextRender) (Utilities|Text|ToText(Float) (Variables|Default|GetHP_Current) "HalfToEven")))

(event Game|Damage|EventAnyDamage
  (params (Damage :type Float%20%28single-precision%29) (DamageType :type Damage%20Type%20Object%20Reference) (InstigatedBy :type Controller%20Object%20Reference) (DamageCauser :type Actor%20Object%20Reference))
  (bind _charactor_dead (CallFunction|ApplyDamage Damage))
  (if _charactor_dead
    (Development|PrintString "I'm dead")))

(event Game|Damage|EventPointDamage
  (params (Damage :type Float%20%28single-precision%29) (DamageType :type Damage%20Type%20Object%20Reference) (HitLocation :type Vector :default "0, 0, 0") (HitNormal :type Vector :default "0, 0, 0") (HitComponent :type Primitive%20Component%20Object%20Reference) (BoneName :type Name :default "None") (ShotFromDirection :type Vector :default "0, 0, 0") (InstigatedBy :type Controller%20Object%20Reference) (DamageCauser :type Actor%20Object%20Reference) (HitInfo :type Hit%20Result%20Structure%20%28by%20ref%29)))

(event Input|ActionEvents|InputActionSprint
  (params (Key :type Key%20Structure :default "None"))
  (:Pressed
    (Variables|/Script/Engine.CharacterMovementComponent|SetMaxWalkSpeed (Variables|Character|GetCharacterMovement) 9e+02))
  (:Released
    (Variables|/Script/Engine.CharacterMovementComponent|SetMaxWalkSpeed (Variables|Character|GetCharacterMovement) 4.5e+02)))

(event Input|ActionEvents|InputActionInteract
  (params (Key :type Key%20Structure :default "None"))
  (bind _lampreference (Variables|Default|GetLampreference))
  (:Pressed
    (Utilities|FlowControl|Sequence
      (:then_0
        (if (Utilities|IsValid (Variables|Default|GetLampreference))
          (Default|SwitchLight _lampreference (not (Variables|/Game/AlexeyOsipov/BluePrints/Character/Intaract/BaseLamp.BaseLamp_C|GetOn/Off _lampreference)))))
      (:then_1
        (if (Utilities|IsValid (Variables|Default|GetWeaponRefInteract))
          (if (Utilities|IsValid (Variables|Default|GetWeaponRefActive))
            (CallFunction|Dropeitem)
            (CallFunction|Takeitem)
            (else
              (CallFunction|Takeitem))))))))

(event Input|ActionEvents|InputActionFire
  (params (Key :type Key%20Structure :default "None"))
  (bind _weaponrefactive (Variables|Default|GetWeaponRefActive))
  (:Pressed
    (if (Utilities|IsValid _weaponrefactive)
      (Default|FireBaseWeapon _weaponrefactive))))

(event Input|ActionEvents|InputActionDropeitem
  (params (Key :type Key%20Structure :default "None"))
  (:Pressed
    (CallFunction|Dropeitem)))

(event Input|ActionEvents|InputActionJump
  (params (Key :type Key%20Structure :default "None"))
  (:Pressed
    (Character|Jump)))

(event Input|AxisEvents|InputAxisMoveForvodr
  (params (AxisValue :type Float%20%28single-precision%29))
  (Pawn|Input|AddMovementInput (Transformation|GetActorForwardVector) AxisValue false))

(event Input|AxisEvents|InputAxisMoveRight
  (params (AxisValue :type Float%20%28single-precision%29))
  (Pawn|Input|AddMovementInput (Transformation|GetActorRightVector) AxisValue false))

(event Input|AxisEvents|InputAxisTurn
  (params (AxisValue :type Float%20%28single-precision%29))
  (Pawn|Input|AddControllerYawInput AxisValue))

(event Input|AxisEvents|InputAxisLookUp
  (params (AxisValue :type Float%20%28single-precision%29))
  (Pawn|Input|AddControllerPitchInput AxisValue))

(fn ConstructionScript)

(fn Dropeitem
  (if (Utilities|IsValid (Variables|Default|GetWeaponRefActive))
    (Transformation|DetachFromActor (Variables|Default|GetWeaponRefActive) "KeepWorld" "KeepWorld" "KeepWorld")
    (Physics|SetSimulatePhysics (Variables|/Game/AlexeyOsipov/Weapon/Baseweapon.BaseWeapon_C|GetStaticMesh (Variables|Default|GetWeaponRefActive)) true)
    (Variables|Default|SetWeaponRefActive 0)))

(fn Takeitem
  (Variables|Default|SetWeaponRefActive (Variables|Default|GetWeaponRefInteract))
  (Transformation|AttachComponentToComponent (Variables|Default|GetWeaponRefActive) (Variables|Default|GetScene) "None" "SnapToTarget" "SnapToTarget" "KeepWorld" true)
  (Physics|SetSimulatePhysics (Variables|/Game/AlexeyOsipov/Weapon/Baseweapon.BaseWeapon_C|GetStaticMesh (Variables|Default|GetWeaponRefInteract)) false)
  (Variables|Default|SetWeaponRefInteract 0))

(fn ApplyDamage
  (params (Damage :type Float%20%28single-precision%29))
  (Variables|Default|SetHP_Current (Math|Float|Clamp(Float) (- (Variables|Default|GetHP_Current) Damage) 0.0 (Variables|Default|GetHP_Max)))
  (return (== (Variables|Default|GetHP_Current) 0.0)))